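; BP_InspectionObject is an interactable physics object that the player can pick up, inspect and snap onto designated actors.
; Interact detaches it and grabs it with the player's PhysicsHandle, briefly ignoring nearby collisions and delaying re-attachment.
; StopInteract releases it and restores collision, while Inspect toggles the player's inspection state, resetting InspectObjectLocation rotation on exit.
; Hitting an actor in PossibleSnapPoints releases and attaches it with that point's offsets.
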(event `self.Interact`
  (params (PlayerReference :type "/Game/TemplateAssets/Blueprints/BP_PlayerCharacter Object Reference"))
  (bind _staticmesh (`self.StaticMesh`))
  (`parent.Interact` PlayerReference)
  ;[1 1 1] Re-enable attachments
  (set `self.CanBeAttached` false)
  (`self.K2_DetachFromActor` "KeepWorld" "KeepWorld" "KeepWorld")
  (`PrimitiveComponent.SetSimulatePhysics` (`self.StaticMesh`) true)
  (set `/Game/TemplateAssets/Blueprints/BP_PlayerCharacter.InteractingObject` self PlayerReference)
  ;[1 1 1] Temporarily disable physics collisions to stop nearby objects from being thrown around
  (`PrimitiveComponent.SetCollisionResponseToChannel` _staticmesh "ECC_PhysicsBody" "ECR_Ignore")
  (`PrimitiveComponent.SetCollisionResponseToChannel` _staticmesh "ECC_WorldDynamic" "ECR_Ignore")
  (`PrimitiveComponent.SetCollisionResponseToChannel` _staticmesh "ECC_GameTraceChannel2" "ECR_Ignore")
  (`PhysicsHandleComponent.GrabComponentAtLocationWithRotation` :`self` (`/Game/TemplateAssets/Blueprints/BP_PlayerCharacter.PhysicsHandle` PlayerReference) :`Component` _staticmesh :`Location` (`SceneComponent.K2_GetComponentLocation` _staticmesh))
  ;[1 1 1] Disable collision with player to avoid being thrown around by the picked up object
  (`PrimitiveComponent.SetCollisionResponseToChannel` _staticmesh "ECC_Pawn" "ECR_Ignore")
  (`KismetSystemLibrary.Delay` 0.1)
  ;[1 1 1] Re-enable physics collisions
  (`PrimitiveComponent.SetCollisionResponseToChannel` _staticmesh "ECC_PhysicsBody" "ECR_Block")
  (`PrimitiveComponent.SetCollisionResponseToChannel` _staticmesh "ECC_WorldDynamic" "ECR_Block")
  (`PrimitiveComponent.SetCollisionResponseToChannel` _staticmesh "ECC_GameTraceChannel2" "ECR_Block")
  (`KismetSystemLibrary.Delay` 1.0)
  ;[1 1 1] Re-enable attachments
  (set `self.CanBeAttached` true))

(event `self.StopInteract`
  (params (PlayerReference :type "/Game/TemplateAssets/Blueprints/BP_PlayerCharacter Object Reference"))
  (bind _staticmesh (`self.StaticMesh`))
  (`parent.StopInteract` PlayerReference)
  (`PhysicsHandleComponent.ReleaseComponent` (`/Game/TemplateAssets/Blueprints/BP_PlayerCharacter.PhysicsHandle` PlayerReference))
  ;[1 1 1] Renable collisions. Failsafe if released too quickly
  (`PrimitiveComponent.SetCollisionResponseToChannel` _staticmesh "ECC_Pawn" "ECR_Block")
  (`PrimitiveComponent.SetCollisionResponseToChannel` _staticmesh "ECC_PhysicsBody" "ECR_Block")
  (`PrimitiveComponent.SetCollisionResponseToChannel` _staticmesh "ECC_WorldDynamic" "ECR_Block")
  (`PrimitiveComponent.SetCollisionResponseToChannel` _staticmesh "ECC_GameTraceChannel2" "ECR_Block")
  (set `/Game/TemplateAssets/Blueprints/BP_PlayerCharacter.InteractingObject` null PlayerReference)
  (set `/Game/TemplateAssets/Blueprints/BP_PlayerCharacter.IsInspectingObject` false PlayerReference))

(event `self.Inspect`
  (params (PlayerReference :type "/Game/TemplateAssets/Blueprints/BP_PlayerCharacter Object Reference"))
  (if (`/Game/TemplateAssets/Blueprints/BP_PlayerCharacter.IsInspectingObject` PlayerReference)
    (`SceneComponent.K2_SetWorldRotation` :`self` (`/Game/TemplateAssets/Blueprints/BP_PlayerCharacter.InspectObjectLocation` PlayerReference))
    (set `/Game/TemplateAssets/Blueprints/BP_PlayerCharacter.IsInspectingObject` false PlayerReference)
    (else
      (set `/Game/TemplateAssets/Blueprints/BP_PlayerCharacter.IsInspectingObject` true PlayerReference))))

(event `self.StaticMesh.OnComponentHit`
  (params (HitComponent :type "PrimitiveComponent Object Reference") (OtherActor :type "Actor Object Reference") (OtherComp :type "PrimitiveComponent Object Reference") (NormalImpulse :type "Vector Structure") (Hit :type "HitResult Structure (by ref)"))
  (for _array_element (`self.PossibleSnapPoints`)
    (bind (_snaptoactor _positionoffset _rotationoffset) (break `/Game/TemplateAssets/Blueprints/UtilityClasses/S_AttachStruct` _array_element))
    (if (and (== OtherActor _snaptoactor) (`KismetSystemLibrary.IsValid` _snaptoactor) (`self.CanBeAttached`))
      (bind _asbp_player_character (cast `/Game/TemplateAssets/Blueprints/BP_PlayerCharacter` (`GameplayStatics.GetPlayerCharacter` 0)))
      (`self.StopInteract` _asbp_player_character)
      (`PrimitiveComponent.SetSimulatePhysics` (`self.StaticMesh`) false)
      (`self.K2_AttachToComponent` (`self.GetComponentByClass` _snaptoactor "/Script/Engine.StaticMeshComponent") "None" "SnapToTarget" "SnapToTarget" "KeepWorld")
      (`self.K2_SetActorRelativeLocation` _positionoffset false true)
      (`self.K2_AddActorLocalRotation` _rotationoffset)
      (break))))

(fn `UserConstructionScript`)
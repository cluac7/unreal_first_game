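; Climbable ladder actor that starts and ends climbing on BP_PlayerCharacter through overlaps with its box collision.
; The construction script builds stacked rung meshes, sizes the box to fit and positions top entry and exit snap points.
; On overlap, it projects the contact point onto the ladder's axes to compute snap positions, using the snap point height near the top.
; Exits away from the top reset rotation and briefly disable CanClimb.
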(event `self.LadderBody.OnComponentBeginOverlap`
  (params (OverlappedComponent :type "PrimitiveComponent Object Reference") (OtherActor :type "Actor Object Reference") (OtherComp :type "PrimitiveComponent Object Reference") (OtherBodyIndex :type Integer) (bFromSweep :type Boolean) (SweepResult :type "HitResult Structure (by ref)"))
  (bind _relativelocation_x (`KismetMathLibrary.BreakVector` (`SceneComponent.RelativeLocation` (`self.LadderTopEntrySnapPoint`))))
  (bind (_relativelocation_x_2 _relativelocation_y _relativelocation_z) (`KismetMathLibrary.BreakVector` (`SceneComponent.RelativeLocation` (`self.LadderTopEntrySnapPoint`))))
  (bind _asbp_player_character (cast `/Game/TemplateAssets/Blueprints/BP_PlayerCharacter` OtherActor))
  (if (`/Game/TemplateAssets/Blueprints/BP_PlayerCharacter.canClimb` _asbp_player_character)
    (bind _playernearladdertop (`/Game/TemplateAssets/Blueprints/BP_PlayerCharacter.CheckIfNearLadderTop` _asbp_player_character self))
    (if _playernearladdertop
      (`/Game/TemplateAssets/Blueprints/BP_PlayerCharacter.StartClimb` _asbp_player_character self (+ (* (`self.GetActorForwardVector`) _relativelocation_x_2) (+ (* (`self.GetActorUpVector`) _relativelocation_z) (`self.K2_GetActorLocation`) (* (`self.GetActorRightVector`) (* (`KismetMathLibrary.Dot_VectorVector` (- (`self.K2_GetActorLocation`) (`KismetMathLibrary.MakeVector` (.x (`.ImpactPoint` (`GameplayStatics.BreakHitResult` SweepResult))) (.y (`.ImpactPoint` (`GameplayStatics.BreakHitResult` SweepResult))) (.z (`.ImpactPoint` (`GameplayStatics.BreakHitResult` SweepResult))))) (`self.GetActorRightVector`)) -1.0)))))
      (else
        (`/Game/TemplateAssets/Blueprints/BP_PlayerCharacter.StartClimb` _asbp_player_character self (+ (* (`self.GetActorForwardVector`) _relativelocation_x) (+ (* (`self.GetActorUpVector`) (* (`KismetMathLibrary.Dot_VectorVector` (- (`self.K2_GetActorLocation`) (`KismetMathLibrary.MakeVector` (.x (`.ImpactPoint` (`GameplayStatics.BreakHitResult` SweepResult))) (.y (`.ImpactPoint` (`GameplayStatics.BreakHitResult` SweepResult))) (.z (`.ImpactPoint` (`GameplayStatics.BreakHitResult` SweepResult))))) (`self.GetActorUpVector`)) -1.0)) (`self.K2_GetActorLocation`) (* (`self.GetActorRightVector`) (* (`KismetMathLibrary.Dot_VectorVector` (- (`self.K2_GetActorLocation`) (`KismetMathLibrary.MakeVector` (.x (`.ImpactPoint` (`GameplayStatics.BreakHitResult` SweepResult))) (.y (`.ImpactPoint` (`GameplayStatics.BreakHitResult` SweepResult))) (.z (`.ImpactPoint` (`GameplayStatics.BreakHitResult` SweepResult))))) (`self.GetActorRightVector`)) -1.0)))))))))

(event `self.LadderBody.OnComponentEndOverlap`
  (params (OverlappedComponent :type "PrimitiveComponent Object Reference") (OtherActor :type "Actor Object Reference") (OtherComp :type "PrimitiveComponent Object Reference") (OtherBodyIndex :type Integer))
  (bind _returnvalue (`self.GetActorRightVector`))
  (bind (_relativelocation_x _relativelocation_y _relativelocation_z) (`KismetMathLibrary.BreakVector` (`SceneComponent.RelativeLocation` (`self.LadderTopExitSnapPoint`))))
  (bind _asbp_player_character (cast `/Game/TemplateAssets/Blueprints/BP_PlayerCharacter` OtherActor))
  (if (`/Game/TemplateAssets/Blueprints/BP_PlayerCharacter.canClimb` _asbp_player_character)
    (bind _playernearladdertop (`/Game/TemplateAssets/Blueprints/BP_PlayerCharacter.CheckIfNearLadderTop` _asbp_player_character self))
    (if _playernearladdertop
      (`/Game/TemplateAssets/Blueprints/BP_PlayerCharacter.EndClimb` _asbp_player_character self (+ (* (`self.GetActorForwardVector`) _relativelocation_x) (* _returnvalue (* (`KismetMathLibrary.Dot_VectorVector` (- (`self.K2_GetActorLocation`) (`self.K2_GetActorLocation` _asbp_player_character)) _returnvalue) -1.0)) (`self.K2_GetActorLocation`) (* (`self.GetActorUpVector`) _relativelocation_z)))
      (else
        (set `/Game/TemplateAssets/Blueprints/BP_PlayerCharacter.canClimb` false _asbp_player_character)
        (`/Game/TemplateAssets/Blueprints/BP_PlayerCharacter.EndClimb` _asbp_player_character self (0.0 0.0 0.0))
        (`/Game/TemplateAssets/Blueprints/BP_PlayerCharacter.ResetRotation` _asbp_player_character)
        (`KismetSystemLibrary.K2_SetTimerDelegate` (delegate `ResetCanClimb`) 0.15)))))

(event `ResetCanClimb`
  (bind _asbp_player_character (cast `/Game/TemplateAssets/Blueprints/BP_PlayerCharacter` (`GameplayStatics.GetPlayerCharacter` 0)))
  (set `/Game/TemplateAssets/Blueprints/BP_PlayerCharacter.canClimb` true _asbp_player_character))

(fn `UserConstructionScript`
  (bind (_collisionboxsize_x _collisionboxsize_y) (`KismetMathLibrary.BreakVector2D` (`self.CollisionBoxSize`)))
  (bind (_topexitpointoffset_x _topexitpointoffset_y) (`KismetMathLibrary.BreakVector2D` (`self.TopExitPointOffset`)))
  (`|ExecutionSequence`
    (:`then_0`
      (for _index (range (`self.LadderRungs`))
        (bind _returnvalue (`AddComponent|NODE_AddStaticMeshComponent-0` :`RelativeTransform` (`KismetMathLibrary.MakeTransform` (`KismetMathLibrary.MakeVector` 0.0 0.0 (* _index (`self.DistanceBetweenRungs`))))))
        (`StaticMeshComponent.SetStaticMesh` _returnvalue (`self.Ladder Mesh`))))
    (:`then_1`
      (`BoxComponent.SetBoxExtent` (`self.LadderBody`) (`KismetMathLibrary.MakeVector` _collisionboxsize_x _collisionboxsize_y (/ (* (`self.LadderRungs`) (`self.DistanceBetweenRungs`)) 2.0)) true)
      (`SceneComponent.K2_SetRelativeLocation` (`self.LadderBody`) (`KismetMathLibrary.MakeVector` (`self.CollisionBoxOffset`) 0.0 (/ (* (- (`self.LadderRungs`) 1) (`self.DistanceBetweenRungs`)) 2.0)) false false))
    (:`then_2`
      (`SceneComponent.K2_SetWorldLocation` (`self.LadderTopEntrySnapPoint`) (+ (`self.K2_GetActorLocation`) (* (`self.GetActorForwardVector`) (`self.PlayerDistanceFromLadder`)) (* (`self.GetActorUpVector`) (* (- (`self.LadderRungs`) 2) (`self.DistanceBetweenRungs`)))) false false)
      (`SceneComponent.K2_SetWorldLocation` (`self.LadderTopExitSnapPoint`) (+ (`self.K2_GetActorLocation`) (* (`self.GetActorForwardVector`) _topexitpointoffset_x) (* (`self.GetActorUpVector`) (+ _topexitpointoffset_y (* (+ (`self.LadderRungs`) 2) (`self.DistanceBetweenRungs`))))) false false))))
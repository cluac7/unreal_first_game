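; Switch-activatable moving object that carries its static mesh along a spline path, optionally combining the path's rotation with the mesh's original rotation.
; The ObjectMovement timeline drives position, with play rate set by travel time and end behavior by movement mode: once, back-and-forth, looping, teleport to start, or reversed variants.
; Deactivation stops it or optionally rewinds it, and Reset restores the timeline start and rotation.
; The construction script sets spline looping and validates switch options.
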(event `self.ReceiveBeginPlay`
  (`parent.ReceiveBeginPlay`)
  (`TimelineComponent.SetPlayRate` (`self.ObjectMovement`) (/ 1.0 (`self.Time`)))
  (set `self.OriginalRotation` (`SceneComponent.K2_GetComponentRotation` (`self.StaticMesh`))))

(event `self.ReceiveTick`
  (params (DeltaSeconds :type "Float (single-precision)"))
  ;[1 1 1] DEBUGGING ONLY - show path direction at each point
)

(event `/Game/TemplateAssets/Blueprints/UtilityClasses/BPI_Activatable.CheckForActivation`
  (params (ActivatedSwitch :type "Actor Object Reference"))
  (`parent.CheckForActivation` ActivatedSwitch))

(event `/Game/TemplateAssets/Blueprints/UtilityClasses/BPI_Resetable.Reset`
  (params (CallingActor :type "Actor Object Reference"))
  (`parent.Reset` CallingActor)
  (`TimelineComponent.SetNewTime` (`self.ObjectMovement`) 0.0)
  (`SceneComponent.K2_SetWorldRotation` (`self.StaticMesh`) (`self.OriginalRotation`) false false))

(event `/Game/TemplateAssets/Blueprints/UtilityClasses/BPI_Activatable.Activate`
  (bind _path (`self.Path`))
  (bind _originalrotation (`self.OriginalRotation`))
  (bind (_movementobjectmode _movementobjecttime) (break `/Game/TemplateAssets/Blueprints/UtilityClasses/S_OverrideStruct` (`self.StructSettings`)))
  (`TimelineComponent.SetPlayRate` (`self.ObjectMovement`) (/ 1.0 _movementobjecttime))
  (set `self.Resetting` false)
  (if (or (`|EnumEquality` _movementobjectmode "NewEnumerator4") (`|EnumEquality` _movementobjectmode "NewEnumerator5"))
    (bind (_direction _time) (`Timeline|ObjectMovement` :!via `Reverse` :!label _label)
      (:`Update`
        (if (`.MovementFollowPathRotation_93_EB131E114101FA36F72437AC2954EBF7` (break `/Game/TemplateAssets/Blueprints/UtilityClasses/S_OverrideStruct` (`self.StructSettings`)))
          (bind _returnvalue (* (`SplineComponent.GetSplineLength` _path) _time))
          (set `self.RotationToApply` (`KismetMathLibrary.ComposeRotators` _originalrotation (`SplineComponent.GetRotationAtDistanceAlongSpline` _path _returnvalue "Local")))
          (else
            (set `self.RotationToApply` _originalrotation)))
        (`SceneComponent.K2_SetWorldLocationAndRotation` (`self.StaticMesh`) (`SplineComponent.GetLocationAtDistanceAlongSpline` _path _returnvalue "World") (`self.RotationToApply`) false false))
      (:`Finished`
        (switch `/Game/TemplateAssets/Blueprints/UtilityClasses/EMoveableStates` (`.MovementObjectMode_72_28E2812E4A4C10D94CD8A99C4802C612` (break `/Game/TemplateAssets/Blueprints/UtilityClasses/S_OverrideStruct` (`self.StructSettings`)))
          (:`NewEnumerator1`
            (if (`self.Resetting`)
              (set `self.Resetting` false)
              (else
                (set `self.PlayReverse` (not (`self.PlayReverse`)))
                (if (`self.PlayReverse`) :!label _label_2
                  (goto _label :!via `Reverse`)
                  (else
                    (goto _label))))))
          (:`NewEnumerator3`
            (if (`self.Resetting`) :!label _label_3
              (set `self.Resetting` false)
              (else
                (goto _label :!via `PlayFromStart`))))
          (:`NewEnumerator0`
            (goto _label_3))
          (:`NewEnumerator5`
            (if (`self.Resetting`) :!label _label_4
              (set `self.Resetting` false)
              (else
                (goto _label :!via `ReverseFromEnd`))))
          (:`NewEnumerator4`
            (goto _label_4)))))
    (else
      (goto _label_2))))

(event `/Game/TemplateAssets/Blueprints/UtilityClasses/BPI_Activatable.Deactivate`
  (bind _objectmovement (`self.ObjectMovement`))
  (bind _movementobjectmode (break `/Game/TemplateAssets/Blueprints/UtilityClasses/S_OverrideStruct` (`self.StructSettings`)))
  (bind (_movementobjectmode_2 _movementobjecttime _movementresetondeactivate) (break `/Game/TemplateAssets/Blueprints/UtilityClasses/S_OverrideStruct` (`self.StructSettings`)))
  (if (`TimelineComponent.IsPlaying` (`self.ObjectMovement`))
    (`TimelineComponent.SetPlayRate` (`self.ObjectMovement`) (/ 1.0 _movementobjecttime) :!label _label_5)
    (if _movementresetondeactivate
      (set `self.Resetting` true)
      (if (or (`|EnumEquality` _movementobjectmode "NewEnumerator4") (`|EnumEquality` _movementobjectmode "NewEnumerator5"))
        (`TimelineComponent.Play` _objectmovement)
        (else
          (`TimelineComponent.Reverse` _objectmovement)))
      (else
        (`TimelineComponent.Stop` _objectmovement)))
    (elif (`|EnumEquality` _movementobjectmode_2 "NewEnumerator2")
      (goto _label_5))))

(fn `SetStructSettings`
  (bind _output_get (set `self.OriginalStruct` (make `/Game/TemplateAssets/Blueprints/UtilityClasses/S_OverrideStruct` (`self.MovementMode`) (`self.Time`) (`self.ResetOnDeactivate`) (`self.FollowPathRotation`))))
  (set `self.StructSettings` _output_get))

(fn `UserConstructionScript`
  (bind _path (`self.Path`))
  (`parent.UserConstructionScript`)
  (`|ExecutionSequence`
    (:`then_0`
      ;[1 1 1] Change the spline to match the selected movement mode
      (switch `/Game/TemplateAssets/Blueprints/UtilityClasses/EMoveableStates` (`self.MovementMode`)
        (:`NewEnumerator2`
          (`SplineComponent.SetClosedLoop` _path false true :!label _label))
        (:`NewEnumerator1`
          (goto _label))
        (:`NewEnumerator0`
          (`SplineComponent.SetClosedLoop` _path true true :!label _label_2))
        (:`NewEnumerator4`
          (goto _label_2))))
    (:`then_1`
      ;[1 1 1] If there are switches in the array, set 'RequiresAllSwitches' to true if 'InSequence' is true.
      ; If there are no switches in the array, deactivate 'RequiresAllSwitches', 'InSequence' and 'ResetOnDeactivate'
      (if (> (`KismetArrayLibrary.Array_Length` (`self.Switches`)) 0)
        (if (`self.InSequence`)
          (set `self.RequiresAllSwitches` true))
        (else
          (set `self.RequiresAllSwitches` false)
          (set `self.InSequence` false)
          (set `self.ResetOnDeactivate` false))))))
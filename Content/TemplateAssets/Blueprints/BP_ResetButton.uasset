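; BP_ResetButton is an overlap-triggered switch that resets a list of assigned actors.
; On overlap it changes to its active colour through a dynamic material instance, sends ResetMessage to each valid actor, and ignores further overlaps until a one-second timer reactivates it.
; At BeginPlay it can attach to another actor's static mesh, keeping world transform and disabling its own mesh collision if that mesh simulates physics.
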(event `self.ReceiveBeginPlay`
  (if (`KismetSystemLibrary.IsValid` (`self.AttachToActor`))
    (`self.K2_AttachToComponent` (`self.GetComponentByClass` (`self.AttachToActor`) "/Script/Engine.StaticMeshComponent") "None" "KeepWorld" "KeepWorld" "KeepWorld")
    (if (`SceneComponent.IsSimulatingPhysics` (`self.GetComponentByClass` (`self.AttachToActor`) "/Script/Engine.StaticMeshComponent") "None")
      (`PrimitiveComponent.SetCollisionEnabled` (`self.StaticMesh`) "NoCollision"))))

(event `self.ReceiveActorBeginOverlap`
  (params (OtherActor :type "Actor Object Reference"))
  (if (not (`self.IsActive`))
    (`self.SetActive` true)
    (set `self.IsActive` true)
    (`KismetSystemLibrary.K2_SetTimerDelegate` (delegate `Reactivate`) 1.0)
    (for _array_element (`self.ActorsToReset`)
      (`/Engine/EditorBlueprintResources/StandardMacros.IsValid` _array_element
        (:`Is Valid`
          (message `/Game/TemplateAssets/Blueprints/UtilityClasses/BPI_Resetable.Reset` _array_element null))))))

(event `Reactivate`
  (`self.SetActive` false)
  (set `self.IsActive` false))

(fn `SetActive`
  (params (Active :type Boolean))
  (bind _switchmaterial (`self.SwitchMaterial`))
  ;[1 1 1] Toggle the switch
  (bind _output_get (set `self.IsActive` Active))
  (if _output_get
    (`MaterialInstanceDynamic.SetVectorParameterValue` _switchmaterial "Colour" (`self.ActivatedColour`))
    (else
      (`MaterialInstanceDynamic.SetVectorParameterValue` _switchmaterial "Colour" (`self.DeactivatedColour`)))))

(fn `UserConstructionScript`
  (bind _returnvalue (`PrimitiveComponent.CreateDynamicMaterialInstance` (`self.StaticMesh`) 0 "/Game/TemplateAssets/Materials/M_Switch.M_Switch" "None"))
  (bind _output_get (set `self.SwitchMaterial` _returnvalue))
  (`MaterialInstanceDynamic.SetVectorParameterValue` _output_get "Colour" (`self.DeactivatedColour`)))
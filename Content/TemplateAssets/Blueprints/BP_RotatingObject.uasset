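; Switch-driven actor, built on a parent activation class, that rotates around a chosen local X, Y or Z axis.
; Activate and Deactivate drive a timeline scaled to the configured duration, which adds delta-time rotation each update, signed by playback direction.
; Finishing applies the mode: once, back-and-forth, or forward/reverse restarts from the original rotation.
; Deactivation either stops it or winds it back; the construction script reconciles switch flags.
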(event `self.ReceiveBeginPlay`
  (`parent.ReceiveBeginPlay`)
  (set `self.OriginalRotation` (`self.K2_GetActorRotation`)))

(event `/Game/TemplateAssets/Blueprints/UtilityClasses/BPI_Resetable.Reset`
  (params (CallingActor :type "Actor Object Reference"))
  (bind _objectrotation (`self.ObjectRotation`))
  (`parent.Reset` CallingActor)
  (`TimelineComponent.SetNewTime` _objectrotation 0.0)
  (`TimelineComponent.Stop` _objectrotation)
  (`self.K2_SetActorRotation` (`self.OriginalRotation`)))

(event `/Game/TemplateAssets/Blueprints/UtilityClasses/BPI_Activatable.CheckForActivation`
  (params (ActivatedSwitch :type "Actor Object Reference"))
  (`parent.CheckForActivation` ActivatedSwitch))

(event `/Game/TemplateAssets/Blueprints/UtilityClasses/BPI_Activatable.Activate`
  (bind _originalrotation (`self.OriginalRotation`))
  (bind _objectrotation (`self.ObjectRotation`))
  (bind _amounttoadd (`self.AmountToAdd`))
  (bind (_movementobjectmode _movementobjecttime _movementresetondeactivate _movementfollowpathrotation _rotationobjectmode) (break `/Game/TemplateAssets/Blueprints/UtilityClasses/S_OverrideStruct` (`self.StructSettings`)))
  (bind (_movementobjectmode_2 _movementobjecttime_2 _movementresetondeactivate_2 _movementfollowpathrotation_2 _rotationobjectmode_2 _rotationobjecttime _rotationobjectvalue) (break `/Game/TemplateAssets/Blueprints/UtilityClasses/S_OverrideStruct` (`self.StructSettings`)))
  (`TimelineComponent.SetPlayRate` (`self.ObjectRotation`) (/ 1.0 (`.RotationObjectTime_79_09F80EF4411CFD8A2EBB01949E47D1D6` (break `/Game/TemplateAssets/Blueprints/UtilityClasses/S_OverrideStruct` (`self.StructSettings`)))))
  ;[1 1 1] Rotation
  (if (or (`|EnumEquality` _rotationobjectmode "NewEnumerator4") (`|EnumEquality` _rotationobjectmode "NewEnumerator5"))
    (if (`.RotationResetOnDeactivate_81_6D3CF1714742FB1B8375B6BBB1375FFC` (break `/Game/TemplateAssets/Blueprints/UtilityClasses/S_OverrideStruct` (`self.StructSettings`)))
      (if (`self.Resetting`)
        (set `self.Resetting` false)
        (`Timeline|ObjectRotation` :!via `Reverse` :!label _label
          (:`Update`
            (set `self.AmountToAdd` (* (* (/ _rotationobjectvalue _rotationobjecttime) (`self.DeltaSeconds`)) (`self.Direction`)))
            (switch `/Game/TemplateAssets/Blueprints/UtilityClasses/ERotationAxis` (`self.RotationDirection`)
              (:`NewEnumerator0`
                (`self.K2_AddActorLocalRotation` (`KismetMathLibrary.MakeRotator` _amounttoadd)))
              (:`NewEnumerator1`
                (`self.K2_AddActorLocalRotation` (`KismetMathLibrary.MakeRotator` 0.0 _amounttoadd)))
              (:`NewEnumerator2`
                (`self.K2_AddActorLocalRotation` (`KismetMathLibrary.MakeRotator` 0.0 0.0 _amounttoadd)))))
          (:`Finished`
            (if (`self.Resetting`)
              (set `self.Resetting` false)
              (`self.K2_SetActorRotation` (`self.OriginalRotation`))
              (else
                (switch `/Game/TemplateAssets/Blueprints/UtilityClasses/EMoveableStates` (`.RotationObjectMode_78_687F58D142AE247738687FB4257C1E46` (break `/Game/TemplateAssets/Blueprints/UtilityClasses/S_OverrideStruct` (`self.StructSettings`)))
                  (:`NewEnumerator1`
                    (if (`self.PlayReverse`)
                      (set `self.PlayReverse` false)
                      (`TimelineComponent.PlayFromStart` _objectrotation)
                      (else
                        (set `self.PlayReverse` true)
                        (`TimelineComponent.ReverseFromEnd` _objectrotation))))
                  (:`NewEnumerator3`
                    (`self.K2_SetActorRotation` _originalrotation :!label _label_2)
                    (`TimelineComponent.PlayFromStart` (`self.ObjectRotation`)))
                  (:`NewEnumerator0`
                    (goto _label_2))
                  (:`NewEnumerator5`
                    (`self.K2_SetActorRotation` _originalrotation :!label _label_3)
                    (`TimelineComponent.ReverseFromEnd` (`self.ObjectRotation`)))
                  (:`NewEnumerator4`
                    (goto _label_3)))))))
        (else
          (set `self.Resetting` false)
          (`self.K2_SetActorRotation` (`self.OriginalRotation`))
          (goto _label :!via `Reverse`)))
      (else
        (set `self.Resetting` false)
        (goto _label :!via `Reverse`)))
    (else
      (set `self.Resetting` false)
      (if (`self.PlayReverse`)
        (goto _label :!via `Reverse`)
        (else
          (goto _label))))))

(event `self.ReceiveTick`
  (params (DeltaSeconds :type "Float (single-precision)"))
  (set `self.DeltaSeconds` DeltaSeconds)
  (if (`TimelineComponent.IsReversing` (`self.ObjectRotation`))
    (set `self.Direction` -1.0)
    (else
      (set `self.Direction` 1.0))))

(event `/Game/TemplateAssets/Blueprints/UtilityClasses/BPI_Activatable.Deactivate`
  (bind _objectrotation (`self.ObjectRotation`))
  (bind (_movementobjectmode _movementobjecttime _movementresetondeactivate _movementfollowpathrotation _rotationobjectmode _rotationobjecttime _rotationobjectvalue _rotationresetondeactivate) (break `/Game/TemplateAssets/Blueprints/UtilityClasses/S_OverrideStruct` (`self.StructSettings`)))
  (bind (_movementobjectmode_2 _movementobjecttime_2 _movementresetondeactivate_2 _movementfollowpathrotation_2 _rotationobjectmode_2) (break `/Game/TemplateAssets/Blueprints/UtilityClasses/S_OverrideStruct` (`self.StructSettings`)))
  (if (`TimelineComponent.IsPlaying` (`self.ObjectRotation`))
    (`TimelineComponent.SetPlayRate` (`self.ObjectRotation`) (/ 1.0 _rotationobjecttime) :!label _label_4)
    (if _rotationresetondeactivate
      (set `self.Resetting` true)
      (if (or (`|EnumEquality` _rotationobjectmode_2 "NewEnumerator4") (`|EnumEquality` _rotationobjectmode_2 "NewEnumerator5"))
        (`TimelineComponent.Play` _objectrotation)
        (else
          (`TimelineComponent.Reverse` _objectrotation)))
      (else
        ;[1 1 1] Stop timelines immediately
        (`TimelineComponent.Stop` (`self.ObjectRotation`))))
    (elif (`|EnumEquality` (`.RotationObjectMode_78_687F58D142AE247738687FB4257C1E46` (break `/Game/TemplateAssets/Blueprints/UtilityClasses/S_OverrideStruct` (`self.StructSettings`))) "NewEnumerator2")
      (goto _label_4))))

(fn `SetStructSettings`
  (bind _output_get (set `self.OriginalStruct` (make `/Game/TemplateAssets/Blueprints/UtilityClasses/S_OverrideStruct` "NewEnumerator2" 0.0 false false (`self.RotationMode`) (`self.RotationTime`) (`self.RotationValue`) (`self.ResetOnDeactivate`))))
  (set `self.StructSettings` _output_get))

(fn `UserConstructionScript`
  (`parent.UserConstructionScript`)
  ;[1 1 1] If there are switches in the array, set 'RequiresAllSwitches' to true  if 'InSequence' is true.
  ; If there are no switches in the array, deactivate 'RequiresAllSwitches', 'InSequence' and 'ResetOnDeactivate'
  (if (> (`KismetArrayLibrary.Array_Length` (`self.Switches`)) 0)
    (if (`self.InSequence`)
      (set `self.RequiresAllSwitches` true))
    (else
      (set `self.RequiresAllSwitches` false)
      (set `self.InSequence` false)
      (set `self.ResetOnDeactivate` false))))
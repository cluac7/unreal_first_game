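; A switch-activated child actor that animates its scale on any combination of X, Y and Z toward a target value.
; One timeline per axis lerps from the original scale, with play rate set by the scale time and repeat behavior by mode (once, back and forth, looping or teleport, including reversed variants).
; Deactivation either stops the timelines or plays them back as a reset, using per-axis flags to suppress repeating.
; SetStructSettings packs the scale variables into the settings struct.
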(event `self.ReceiveBeginPlay`
  (`parent.ReceiveBeginPlay`)
  (bind _output_get (set `self.OriginalScale` (`self.GetActorScale3D`)))
  (set `self.ScaleToApply` _output_get))

(event `/Game/TemplateAssets/Blueprints/UtilityClasses/BPI_Activatable.CheckForActivation`
  (params (ActivatedSwitch :type "Actor Object Reference"))
  (`parent.CheckForActivation` ActivatedSwitch))

(event `/Game/TemplateAssets/Blueprints/UtilityClasses/BPI_Resetable.Reset`
  (params (CallingActor :type "Actor Object Reference"))
  (`parent.Reset` CallingActor)
  (`TimelineComponent.SetNewTime` (`self.ObjectScaleX`) 0.0)
  (`TimelineComponent.SetNewTime` (`self.ObjectScaleY`) 0.0)
  (`TimelineComponent.SetNewTime` (`self.ObjectScaleZ`) 0.0)
  (`self.SetActorScale3D` (`self.OriginalScale`)))

(event `/Game/TemplateAssets/Blueprints/UtilityClasses/BPI_Activatable.Activate`
  (bind _originalscale_x (`KismetMathLibrary.BreakVector` (`self.OriginalScale`)))
  (bind (_scaletoapply_x _scaletoapply_y _scaletoapply_z) (`KismetMathLibrary.BreakVector` (`self.ScaleToApply`)))
  (bind (_originalscale_x_2 _originalscale_y) (`KismetMathLibrary.BreakVector` (`self.OriginalScale`)))
  (bind (_scaletoapply_x_2 _scaletoapply_y_2 _scaletoapply_z_2) (`KismetMathLibrary.BreakVector` (`self.ScaleToApply`)))
  (bind (_originalscale_x_3 _originalscale_y_2 _originalscale_z) (`KismetMathLibrary.BreakVector` (`self.OriginalScale`)))
  (bind (_scaletoapply_x_3 _scaletoapply_y_3) (`KismetMathLibrary.BreakVector` (`self.ScaleToApply`)))
  (bind (_movementobjectmode _movementobjecttime _movementresetondeactivate _movementfollowpathrotation _rotationobjectmode _rotationobjecttime _rotationobjectvalue _rotationresetondeactivate _rotationobjectx _rotationobjecty _rotationobjectz _scaleobjectmode _scaleobjecttime _scaleobjectvalue _scaleresetondeactivate _scaleobjectx) (break `/Game/TemplateAssets/Blueprints/UtilityClasses/S_OverrideStruct` (`self.StructSettings`)))
  (bind (_movementobjectmode_2 _movementobjecttime_2 _movementresetondeactivate_2 _movementfollowpathrotation_2 _rotationobjectmode_2 _rotationobjecttime_2 _rotationobjectvalue_2 _rotationresetondeactivate_2 _rotationobjectx_2 _rotationobjecty_2 _rotationobjectz_2 _scaleobjectmode_2 _scaleobjecttime_2 _scaleobjectvalue_2 _scaleresetondeactivate_2 _scaleobjectx_2 _scaleobjecty) (break `/Game/TemplateAssets/Blueprints/UtilityClasses/S_OverrideStruct` (`self.StructSettings`)))
  (bind (_movementobjectmode_3 _movementobjecttime_3 _movementresetondeactivate_3 _movementfollowpathrotation_3 _rotationobjectmode_3 _rotationobjecttime_3 _rotationobjectvalue_3 _rotationresetondeactivate_3 _rotationobjectx_3 _rotationobjecty_3 _rotationobjectz_3 _scaleobjectmode_3 _scaleobjecttime_3 _scaleobjectvalue_3 _scaleresetondeactivate_3 _scaleobjectx_3 _scaleobjecty_2 _scaleobjectz) (break `/Game/TemplateAssets/Blueprints/UtilityClasses/S_OverrideStruct` (`self.StructSettings`)))
  (`TimelineComponent.SetPlayRate` (`self.ObjectScaleX`) (/ 1.0 (`.ScaleObjectTime_86_433B99C049E8E96568625B8E699CD1B7` (break `/Game/TemplateAssets/Blueprints/UtilityClasses/S_OverrideStruct` (`self.StructSettings`)))))
  (`TimelineComponent.SetPlayRate` (`self.ObjectScaleY`) (/ 1.0 (`.ScaleObjectTime_86_433B99C049E8E96568625B8E699CD1B7` (break `/Game/TemplateAssets/Blueprints/UtilityClasses/S_OverrideStruct` (`self.StructSettings`)))))
  (`TimelineComponent.SetPlayRate` (`self.ObjectScaleZ`) (/ 1.0 (`.ScaleObjectTime_86_433B99C049E8E96568625B8E699CD1B7` (break `/Game/TemplateAssets/Blueprints/UtilityClasses/S_OverrideStruct` (`self.StructSettings`)))))
  (set `self.ResettingX` false)
  (set `self.ResettingY` false)
  (set `self.ResettingZ` false)
  (`|ExecutionSequence`
    (:`then_0`
      ;[1 1 1] Scale X
      (if _scaleobjectx
        (if (or (`|EnumEquality` _scaleobjectmode "NewEnumerator4") (`|EnumEquality` _scaleobjectmode "NewEnumerator5"))
          (bind (_direction _time) (`Timeline|ObjectScaleX` :!via `Reverse` :!label _label)
            (:`Update`
              (bind _output_get (set `self.ScaleToApply` (`KismetMathLibrary.MakeVector` (`KismetMathLibrary.Lerp` _originalscale_x (`.ScaleObjectValue_87_68FEACFE47BFEAAE4835A3A9A2791B53` (break `/Game/TemplateAssets/Blueprints/UtilityClasses/S_OverrideStruct` (`self.StructSettings`))) _time) _scaletoapply_y _scaletoapply_z)))
              (`self.SetActorScale3D` _output_get))
            (:`Finished`
              (switch `/Game/TemplateAssets/Blueprints/UtilityClasses/EMoveableStates` (`.ScaleObjectMode_85_3A2EF0874617966946DB3DA1D4A881DC` (break `/Game/TemplateAssets/Blueprints/UtilityClasses/S_OverrideStruct` (`self.StructSettings`)))
                (:`NewEnumerator1`
                  (if (`self.ResettingX`)
                    (set `self.ResettingX` false)
                    (else
                      (set `self.PlayReverseX` (not (`self.PlayReverseX`)))
                      (if (`self.PlayReverseX`) :!label _label_2
                        (goto _label :!via `Reverse`)
                        (else
                          (goto _label))))))
                (:`NewEnumerator3`
                  (if (`self.ResettingX`) :!label _label_3
                    (set `self.ResettingX` false)
                    (else
                      (goto _label :!via `PlayFromStart`))))
                (:`NewEnumerator0`
                  (goto _label_3))
                (:`NewEnumerator5`
                  (if (`self.ResettingX`) :!label _label_4
                    (set `self.ResettingX` false)
                    (else
                      (goto _label :!via `ReverseFromEnd`))))
                (:`NewEnumerator4`
                  (goto _label_4)))))
          (else
            (goto _label_2)))
        (else
          (goto _label :!via `Stop`))))
    (:`then_1`
      ;[1 1 1] Scale Y
      (if _scaleobjecty
        (if (or (`|EnumEquality` _scaleobjectmode_2 "NewEnumerator4") (`|EnumEquality` _scaleobjectmode_2 "NewEnumerator5"))
          (bind (_direction_2 _time_2) (`Timeline|ObjectScaleY` :!via `Reverse` :!label _label_5)
            (:`Update`
              (bind _output_get_2 (set `self.ScaleToApply` (`KismetMathLibrary.MakeVector` _scaletoapply_x_2 (`KismetMathLibrary.Lerp` _originalscale_y (`.ScaleObjectValue_87_68FEACFE47BFEAAE4835A3A9A2791B53` (break `/Game/TemplateAssets/Blueprints/UtilityClasses/S_OverrideStruct` (`self.StructSettings`))) _time_2) _scaletoapply_z_2)))
              (`self.SetActorScale3D` _output_get_2))
            (:`Finished`
              (switch `/Game/TemplateAssets/Blueprints/UtilityClasses/EMoveableStates` (`.ScaleObjectMode_85_3A2EF0874617966946DB3DA1D4A881DC` (break `/Game/TemplateAssets/Blueprints/UtilityClasses/S_OverrideStruct` (`self.StructSettings`)))
                (:`NewEnumerator1`
                  (if (`self.ResettingY`)
                    (set `self.ResettingY` false)
                    (else
                      (set `self.PlayReverseY` (not (`self.PlayReverseY`)))
                      (if (`self.PlayReverseY`) :!label _label_6
                        (goto _label_5 :!via `Reverse`)
                        (else
                          (goto _label_5))))))
                (:`NewEnumerator3`
                  (if (`self.ResettingY`) :!label _label_7
                    (set `self.ResettingY` false)
                    (else
                      (goto _label_5 :!via `PlayFromStart`))))
                (:`NewEnumerator0`
                  (goto _label_7))
                (:`NewEnumerator5`
                  (if (`self.ResettingY`) :!label _label_8
                    (set `self.ResettingY` false)
                    (else
                      (goto _label_5 :!via `ReverseFromEnd`))))
                (:`NewEnumerator4`
                  (goto _label_8)))))
          (else
            (goto _label_6)))
        (else
          (goto _label_5 :!via `Stop`))))
    (:`then_2`
      ;[1 1 1] Scale Z
      (if _scaleobjectz
        (if (or (`|EnumEquality` _scaleobjectmode_3 "NewEnumerator4") (`|EnumEquality` _scaleobjectmode_3 "NewEnumerator5"))
          (bind (_direction_3 _time_3) (`Timeline|ObjectScaleZ` :!via `Reverse` :!label _label_9)
            (:`Update`
              (bind _output_get_3 (set `self.ScaleToApply` (`KismetMathLibrary.MakeVector` _scaletoapply_x_3 _scaletoapply_y_3 (`KismetMathLibrary.Lerp` _originalscale_z (`.ScaleObjectValue_87_68FEACFE47BFEAAE4835A3A9A2791B53` (break `/Game/TemplateAssets/Blueprints/UtilityClasses/S_OverrideStruct` (`self.StructSettings`))) _time_3))))
              (`self.SetActorScale3D` _output_get_3))
            (:`Finished`
              (switch `/Game/TemplateAssets/Blueprints/UtilityClasses/EMoveableStates` (`.ScaleObjectMode_85_3A2EF0874617966946DB3DA1D4A881DC` (break `/Game/TemplateAssets/Blueprints/UtilityClasses/S_OverrideStruct` (`self.StructSettings`)))
                (:`NewEnumerator1`
                  (if (`self.ResettingZ`)
                    (set `self.ResettingZ` false)
                    (else
                      (set `self.PlayReverseZ` (not (`self.PlayReverseZ`)))
                      (if (`self.PlayReverseZ`) :!label _label_10
                        (goto _label_9 :!via `Reverse`)
                        (else
                          (goto _label_9))))))
                (:`NewEnumerator3`
                  (if (`self.ResettingZ`) :!label _label_11
                    (set `self.ResettingZ` false)
                    (else
                      (goto _label_9 :!via `PlayFromStart`))))
                (:`NewEnumerator0`
                  (goto _label_11))
                (:`NewEnumerator5`
                  (if (`self.ResettingZ`) :!label _label_12
                    (set `self.ResettingZ` false)
                    (else
                      (goto _label_9 :!via `ReverseFromEnd`))))
                (:`NewEnumerator4`
                  (goto _label_12)))))
          (else
            (goto _label_10)))
        (else
          (goto _label_9 :!via `Stop`))))))

(event `/Game/TemplateAssets/Blueprints/UtilityClasses/BPI_Activatable.Deactivate`
  (bind _objectscalex (`self.ObjectScaleX`))
  (bind _objectscaley (`self.ObjectScaleY`))
  (bind _objectscalez (`self.ObjectScaleZ`))
  (bind (_movementobjectmode _movementobjecttime _movementresetondeactivate _movementfollowpathrotation _rotationobjectmode _rotationobjecttime _rotationobjectvalue _rotationresetondeactivate _rotationobjectx _rotationobjecty _rotationobjectz _scaleobjectmode _scaleobjecttime _scaleobjectvalue _scaleresetondeactivate) (break `/Game/TemplateAssets/Blueprints/UtilityClasses/S_OverrideStruct` (`self.StructSettings`)))
  (bind (_movementobjectmode_2 _movementobjecttime_2 _movementresetondeactivate_2 _movementfollowpathrotation_2 _rotationobjectmode_2 _rotationobjecttime_2 _rotationobjectvalue_2 _rotationresetondeactivate_2 _rotationobjectx_2 _rotationobjecty_2 _rotationobjectz_2 _scaleobjectmode_2 _scaleobjecttime_2 _scaleobjectvalue_2 _scaleresetondeactivate_2 _scaleobjectx _scaleobjecty _scaleobjectz) (break `/Game/TemplateAssets/Blueprints/UtilityClasses/S_OverrideStruct` (`self.StructSettings`)))
  (bind _returnvalue (or (`|EnumEquality` _scaleobjectmode_2 "NewEnumerator4") (`|EnumEquality` _scaleobjectmode_2 "NewEnumerator5")))
  (if (or (`TimelineComponent.IsPlaying` (`self.ObjectScaleX`)) (`TimelineComponent.IsPlaying` (`self.ObjectScaleY`)) (`TimelineComponent.IsPlaying` (`self.ObjectScaleZ`)))
    (`TimelineComponent.SetPlayRate` (`self.ObjectScaleX`) (/ 1.0 _scaleobjecttime) :!label _label_13)
    (`TimelineComponent.SetPlayRate` (`self.ObjectScaleY`) (/ 1.0 _scaleobjecttime))
    (`TimelineComponent.SetPlayRate` (`self.ObjectScaleZ`) (/ 1.0 _scaleobjecttime))
    (if _scaleresetondeactivate
      (set `self.ResettingX` true)
      (set `self.ResettingY` true)
      (set `self.ResettingZ` true)
      (`|ExecutionSequence`
        (:`then_0`
          (if _scaleobjectx
            (if _returnvalue
              (`TimelineComponent.Play` _objectscalex)
              (else
                (`TimelineComponent.Reverse` _objectscalex)))))
        (:`then_1`
          (if _scaleobjecty
            (if _returnvalue
              (`TimelineComponent.Play` _objectscaley)
              (else
                (`TimelineComponent.Reverse` _objectscaley)))))
        (:`then_2`
          (if _scaleobjectz
            (if _returnvalue
              (`TimelineComponent.Play` _objectscalez)
              (else
                (`TimelineComponent.Reverse` _objectscalez))))))
      (else
        ;[1 1 1] Stop all timelines immediately
        (`|ExecutionSequence`
          (:`then_0`
            (`TimelineComponent.Stop` (`self.ObjectScaleX`)))
          (:`then_1`
            (`TimelineComponent.Stop` (`self.ObjectScaleY`)))
          (:`then_2`
            (`TimelineComponent.Stop` (`self.ObjectScaleZ`))))))
    (elif (`|EnumEquality` (`.ScaleObjectMode_85_3A2EF0874617966946DB3DA1D4A881DC` (break `/Game/TemplateAssets/Blueprints/UtilityClasses/S_OverrideStruct` (`self.StructSettings`))) "NewEnumerator2")
      (goto _label_13))))

(fn `SetStructSettings`
  (bind _output_get (set `self.OriginalStruct` (make `/Game/TemplateAssets/Blueprints/UtilityClasses/S_OverrideStruct` "NewEnumerator2" 0.0 false false "NewEnumerator2" 0.0 0.0 false false false false (`self.ScaleMode`) (`self.ScaleTime`) (`self.ScaleValue`) (`self.ResetOnDeactivate`) (`self.ScaleX`) (`self.ScaleY`) (`self.ScaleZ`))))
  (set `self.StructSettings` _output_get))

(fn `UserConstructionScript`
  (`parent.UserConstructionScript`)
  ;[1 1 1] If there are switches in the array, set 'RequiresAllSwitches' to true and 'ResetOnDeactivate' to false if 'InSequence' is true.
  ; If there are no switches in the array, deactivate 'RequiresAllSwitches', 'InSequence' and 'ResetOnDeactivate'
  (if (> (`KismetArrayLibrary.Array_Length` (`self.Switches`)) 0)
    (if (`self.InSequence`)
      (set `self.RequiresAllSwitches` true)
      (set `self.ResetOnDeactivate` false))
    (else
      (set `self.RequiresAllSwitches` false)
      (set `self.InSequence` false)
      (set `self.ResetOnDeactivate` false))))
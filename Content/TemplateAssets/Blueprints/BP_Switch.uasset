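; Overlap-triggered switch that toggles or acts as a pressure plate, recolours its dynamic material and calls CallOnActivate on each state change.
; Overlap events honour options for required actors (keycard-style), staying active, objects that must remain and timed deactivation.
; A brief re-trigger lockout prevents double activation when it is attached to moving actors.
; Reset deactivates it and messages the calling actor to remove it from its input sequence.
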(event `self.ReceiveBeginPlay`
  (if (`KismetSystemLibrary.IsValid` (`self.AttachToActor`))
    (`self.K2_AttachToComponent` (`self.GetComponentByClass` (`self.AttachToActor`) "/Script/Engine.StaticMeshComponent") "None" "KeepWorld" "KeepWorld" "KeepWorld")
    (if (`SceneComponent.IsSimulatingPhysics` (`self.GetComponentByClass` (`self.AttachToActor`) "/Script/Engine.StaticMeshComponent") "None")
      (`PrimitiveComponent.SetCollisionEnabled` (`self.StaticMesh`) "NoCollision"))))

(event `self.ReceiveActorBeginOverlap`
  (params (OtherActor :type "Actor Object Reference"))
  (if (`self.AllowActivation`)
    (`|ExecutionSequence`
      (:`then_0`
        ;[1 1 1] Small delay necessary to prevent collision from triggering twice on the same physics substep (for switches attached to moving objects)
        (set `self.AllowActivation` false)
        (`KismetSystemLibrary.Delay` 0.2)
        (set `self.AllowActivation` true))
      (:`then_1`
        ;[1 1 1] If the switch should remain active once activated, do not activate again.
        (if (not (and (`self.StayActive`) (`self.IsActive`)))
          ;[1 1 1] Does this switch require a specific actor(s) to activate it (like a keycard)?
          (if (> (`KismetArrayLibrary.Array_Length` (`self.RequiredActors`)) 0)
            ;[1 1 1] If specific actors are required, did one of those actors trigger this event?
            (if (!= (`KismetArrayLibrary.Array_Find` (`self.RequiredActors`) OtherActor) -1)
              ;[1 1 1] Does this switch require an object (specific or not) to stay in the area (like a weighted pressure plate)?
              (if (`self.ObjectMustStay`) :!label _label
                ;[1 1 1] Activate switch - don't start timer
                (`self.SetActive` true)
                (else
                  ;[1 1 1] Toggle the switch
                  (bind _output_get (set `self.IsActive` (not (`self.IsActive`))))
                  (`self.SetActive` _output_get)
                  ;[1 1 1] If a timer duration has been set, turn the switch back off
                  (if (> (`self.ActivatedDuration`) 0.0)
                    (`KismetSystemLibrary.K2_SetTimerDelegate` (delegate `TimedDeactivate`) (`self.ActivatedDuration`) :!label _label_2)))))
            (else
              (goto _label))))))))

(event `TimedDeactivate`
  (bind _overlappingactors (`PrimitiveComponent.GetOverlappingActors` (`self.Box`) null))
  (if (> (`KismetArrayLibrary.Array_Length` (`self.RequiredActors`)) 0)
    ;[1 1 1] Check if the required object hasn't been put back into place
    (if (> (`KismetArrayLibrary.Array_Length` _overlappingactors) 0)
      (for _array_element _overlappingactors
        (if (> (`KismetArrayLibrary.Array_Find` (`self.RequiredActors`) _array_element) -1)
          (set `self.RequiredActorFound` true)
          (break)
          (else
            (set `self.RequiredActorFound` false))))
      (if (not (`self.RequiredActorFound`))
        (`self.SetActive` false :!label _label_3))
      (else
        (goto _label_3)))
    (else
      (goto _label_3))))

(event `self.ReceiveActorEndOverlap`
  (params (OtherActor :type "Actor Object Reference"))
  (bind _overlappingactors (`PrimitiveComponent.GetOverlappingActors` (`self.Box`) null))
  (if (`self.AllowActivation`)
    ;[1 1 1] If the switch should remain active once activated, do not deactivate.
    (if (not (and (`self.StayActive`) (`self.IsActive`)))
      ;[1 1 1] Does this switch require a specific actor(s) to activate it (like a keycard)?
      (if (> (`KismetArrayLibrary.Array_Length` (`self.RequiredActors`)) 0)
        ;[1 1 1] Are there no other objects still within the collider?
        (if (> (`KismetArrayLibrary.Array_Length` _overlappingactors) 0)
          (set `self.RequiredActorFound` false)
          ;[1 1 1] If specific actors are required, is one still within the collision box?
          (for _array_element _overlappingactors
            (if (> (`KismetArrayLibrary.Array_Find` (`self.RequiredActors`) _array_element) -1)
              (set `self.RequiredActorFound` true)
              (break)
              (else
                (set `self.RequiredActorFound` false))))
          (if (not (`self.RequiredActorFound`))
            ;[1 1 1] Does this switch require an object (specific or not) to stay in the area (like a weighted pressure plate)?
            (if (`self.ObjectMustStay`) :!label _label_4
              ;[1 1 1] If a timer duration has been set, turn the switch back off
              (if (> (`self.ActivatedDuration`) 0.0)
                (goto _label_2)
                (else
                  ;[1 1 1] Deactivate switch immediately
                  (`self.SetActive` false)))))
          (else
            (goto _label_4)))
        (else
          ;[1 1 1] Are there no other objects still within the collider?
          (if (== (`KismetArrayLibrary.Array_Length` (`PrimitiveComponent.GetOverlappingActors` (`self.Box`) null)) 0)
            (goto _label_4)))))))

(event `/Game/TemplateAssets/Blueprints/UtilityClasses/BPI_Resetable.Reset`
  (params (CallingActor :type "Actor Object Reference"))
  (`self.SetActive` false)
  (`self.RemoveSelfFromInputSequence` CallingActor)
  (set `self.AllowActivation` true))

(event `AddSequenceActor`
  (params (ActorToAdd :type "Actor Object Reference"))
  (`KismetArrayLibrary.Array_Add` (`self.SequenceActors`) ActorToAdd))

(event `RemoveSelfFromInputSequence`
  (params (RemoveFromActor :type "Actor Object Reference"))
  (message `/Game/TemplateAssets/Blueprints/UtilityClasses/BPI_Activatable.RemoveFromInputSequence` RemoveFromActor self))

(fn `SetActive`
  (params (Active :type Boolean))
  (bind _switchmaterial (`self.SwitchMaterial`))
  ;[1 1 1] Toggle the switch
  (bind _output_get (set `self.IsActive` Active))
  (if _output_get
    (`MaterialInstanceDynamic.SetVectorParameterValue` _switchmaterial "Colour" (`self.ActivatedColour`))
    (else
      (`MaterialInstanceDynamic.SetVectorParameterValue` _switchmaterial "Colour" (`self.DeactivatedColour`))))
  (`self.OnActivate` self))

(fn `UserConstructionScript`
  (bind _returnvalue (`PrimitiveComponent.CreateDynamicMaterialInstance` (`self.StaticMesh`) 0 "/Game/TemplateAssets/Materials/M_Switch.M_Switch" "None"))
  (bind _output_get (set `self.SwitchMaterial` _returnvalue))
  (`MaterialInstanceDynamic.SetVectorParameterValue` _output_get "Colour" (`self.DeactivatedColour`))
  (if (`self.StayActive`)
    (set `self.ObjectMustStay` false)
    (set `self.ActivatedDuration` 0.0)))
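; BP_WinZone is a trigger zone that wins the level when every actor in its WinningActors list is inside it.
; A boolean array parallel to that list is set on begin overlap and cleared when the Box component's overlap ends.
; Each begin overlap runs CheckForWin, which shows WBP_WinScreen if all flags are true, then reloads the current level after a short delay.
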(event `self.ReceiveBeginPlay`
  (for _ (`self.WinningActors`)
    (`KismetArrayLibrary.Array_Add` (`self.RequiredActors`))))

(event `self.ReceiveActorBeginOverlap`
  (params (OtherActor :type "Actor Object Reference"))
  (for (_array_element _array_index) (`self.WinningActors`)
    (if (== _array_element OtherActor)
      (`KismetArrayLibrary.Array_Set` (`self.RequiredActors`) _array_index true)
      (break)))
  (`self.CheckForWin`))

(event `self.Box.OnComponentEndOverlap`
  (params (OverlappedComponent :type "PrimitiveComponent Object Reference") (OtherActor :type "Actor Object Reference") (OtherComp :type "PrimitiveComponent Object Reference") (OtherBodyIndex :type Integer))
  (for (_array_element _array_index) (`self.WinningActors`)
    (if (== _array_element OtherActor)
      (`KismetArrayLibrary.Array_Set` (`self.RequiredActors`) _array_index))))

(event `CheckForWin`
  (for _array_element (`self.RequiredActors`)
    (if _array_element
      (set `self.WinConditionMet` true)
      (else
        (set `self.WinConditionMet` false)
        (break))))
  (if (`self.WinConditionMet`)
    (bind _returnvalue (`|CreateWidget` "/Game/TemplateAssets/Widgets/WBP_WinScreen.WBP_WinScreen_C"))
    (`UserWidget.AddToViewport` _returnvalue 0)
    (`KismetSystemLibrary.Delay` 3.0)
    (bind _returnvalue_2 (`GameplayStatics.GetCurrentLevelName` true))
    (`GameplayStatics.OpenLevel` (`KismetStringLibrary.Conv_StringToName` _returnvalue_2))))

(fn `UserConstructionScript`)
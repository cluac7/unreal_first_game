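; BP_enemy is an enemy actor that advances in steps and ends the game if it hits the killable character.
; A looping timer set on BeginPlay calls MoveForward, which sweeps the actor by a world offset only while the referenced TriggerBox_Blueprint reports PlayerIn.
; On a hit it prints a debug message, then quits the game for KillableChar or destroys itself for anything else.
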(event `self.ReceiveBeginPlay`
  (`KismetSystemLibrary.K2_SetTimerDelegate` (delegate `move_forward_event`) 1.0 true))

(event `move_forward_event`
  (`self.move_forward`))

(event `self.ReceiveHit`
  (params (MyComp :type "PrimitiveComponent Object Reference") (Other :type "Actor Object Reference") (OtherComp :type "PrimitiveComponent Object Reference") (bSelfMoved :type Boolean) (HitLocation :type "Vector Structure") (HitNormal :type "Vector Structure") (NormalImpulse :type "Vector Structure") (Hit :type "HitResult Structure (by ref)"))
  (`KismetSystemLibrary.PrintString` "collided")
  (if (== Other (`self.killable_char`))
    (`KismetSystemLibrary.QuitGame` null "Quit")
    (else
      (`self.K2_DestroyActor`))))

(event `self.ReceiveTick`
  (params (DeltaSeconds :type "Float (single-precision)")))

(fn `move_forward`
  (bind _astrigger_box_blueprint (cast `/Game/TemplateAssets/Blueprints/TriggerBox_Blueprint` (`self.trigger box`)))
  (if (`/Game/TemplateAssets/Blueprints/TriggerBox_Blueprint.player in` _astrigger_box_blueprint)
    (`self.K2_AddActorWorldOffset` (`self.delta_location`) true)))

(fn `UserConstructionScript`)
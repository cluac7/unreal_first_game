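; Base Blueprint for switch-driven activatable actors, which can attach to another actor's static mesh at begin play and activate immediately if no switches are assigned.
; It binds to BP_Switch activation events and calls Activate or Deactivate when any switch, all switches, or an ordered sequence is satisfied.
; Active switches can override its settings struct.
; Sequence input is checked after a short delay, resetting switches on a wrong order.
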(event `self.ReceiveBeginPlay`
  (`self.SetStructSettings`)
  (`|ExecutionSequence`
    (:`then_0`
      (if (`KismetSystemLibrary.IsValid` (`self.AttachToActor`))
        (`self.K2_AttachToComponent` (`self.GetComponentByClass` (`self.AttachToActor`) "/Script/Engine.StaticMeshComponent") "None" "KeepWorld" "KeepWorld" "KeepWorld")))
    (:`then_1`
      (if (> (`KismetArrayLibrary.Array_Length` (`self.Switches`)) 0)
        (for _array_element (`self.Switches`)
          (bind _asbp_switch (cast `/Game/TemplateAssets/Blueprints/BP_Switch` _array_element)
            (:`then`
              (add `/Game/TemplateAssets/Blueprints/BP_Switch.OnActivate` _asbp_switch (delegate `self.CheckForActivation`))
              (if (`self.InSequence`)
                (`/Game/TemplateAssets/Blueprints/BP_Switch.AddSequenceActor` _asbp_switch self)
                (set `/Game/TemplateAssets/Blueprints/BP_Switch.StayActive` true _asbp_switch)))
            (:`CastFailed`
              (`KismetSystemLibrary.PrintString` (`KismetStringLibrary.Concat_StrStr` "Actor that is not a BP_Switch found in " (`KismetSystemLibrary.GetObjectName` self) " Switches array") true true (struct :`R` 1.0 :`A` 1.0) 60.0))))
        (else
          (`self.Activate`))))))

(event `self.CheckForActivation`
  (params (ActivatedSwitch :type "Actor Object Reference"))
  (bind _asbp_switch (cast `/Game/TemplateAssets/Blueprints/BP_Switch` ActivatedSwitch))
  (if (`/Game/TemplateAssets/Blueprints/BP_Switch.IsActive` _asbp_switch)
    (if (`/Game/TemplateAssets/Blueprints/BP_Switch.EnableOverride` _asbp_switch)
      (set `self.StructSettings` (`/Game/TemplateAssets/Blueprints/BP_Switch.OverrideSettings` _asbp_switch))
      (else
        (set `self.StructSettings` (`self.OriginalStruct`)))))
  (if (`self.RequiresAllSwitches`)
    ;[1 1 1] Switches must be activate in the correct sequence
    (if (`self.InSequence`)
      (bind _asbp_switch_2 (cast `/Game/TemplateAssets/Blueprints/BP_Switch` ActivatedSwitch))
      (if (`/Game/TemplateAssets/Blueprints/BP_Switch.IsActive` _asbp_switch_2)
        (`KismetArrayLibrary.Array_Add` (`self.InputSequence`) _asbp_switch_2)
        (if (== (`KismetArrayLibrary.Array_Length` (`self.InputSequence`)) (`KismetArrayLibrary.Array_Length` (`self.Switches`)))
          (`self.CheckSeqeuence`)))
      (else
        ;[1 1 1] All switches must be active
        (for _array_element (`self.Switches`)
          (bind _asbp_switch_3 (cast `/Game/TemplateAssets/Blueprints/BP_Switch` _array_element))
          (if (`/Game/TemplateAssets/Blueprints/BP_Switch.IsActive` _asbp_switch_3)
            (set `self.RequiredSwitchesActive` true)
            (else
              (set `self.RequiredSwitchesActive` false)
              (break))))
        (if (`self.RequiredSwitchesActive`)
          (`self.Activate`)
          (else
            (`self.Deactivate`)))))
    (else
      ;[1 1 1] Only one switch needs to be active
      (set `self.RequiredSwitchesActive` false)
      (for _array_element_2 (`self.Switches`)
        (bind _asbp_switch_4 (cast `/Game/TemplateAssets/Blueprints/BP_Switch` _array_element_2))
        (if (`/Game/TemplateAssets/Blueprints/BP_Switch.IsActive` _asbp_switch_4)
          (set `self.RequiredSwitchesActive` true)
          (break)))
      (if (`self.RequiredSwitchesActive`)
        (`self.Activate`)
        (else
          (`self.Deactivate`))))))

(event `self.ResetSwitches`
  (params (ResetArray :type "Array of Actor Object Reference (by ref)"))
  (for _array_element ResetArray
    (bind _asbp_switch (cast `/Game/TemplateAssets/Blueprints/BP_Switch` _array_element))
    (bind _output_get (set `/Game/TemplateAssets/Blueprints/BP_Switch.IsActive` false _asbp_switch))
    (`/Game/TemplateAssets/Blueprints/BP_Switch.SetActive` _asbp_switch _output_get)))

(event `self.CheckSeqeuence`
  (bind _inputsequence (`self.InputSequence`))
  ;[1 1 1] Must have a small delay to wait for all objects checking the sequence to update their input sequence
  (`KismetSystemLibrary.Delay` 0.2)
  (for (_array_element _array_index) (`self.InputSequence`)
    (if (== _array_element (`|GetArrayItem` (`self.Switches`) _array_index))
      (set `self.RequiredSwitchesActive` true)
      (else
        (set `self.RequiredSwitchesActive` false)
        (`self.ResetSwitches` _inputsequence)
        (`KismetArrayLibrary.Array_Clear` _inputsequence)
        (break))))
  (if (`self.RequiredSwitchesActive`)
    (`self.Activate`)))

(event `/Game/TemplateAssets/Blueprints/UtilityClasses/BPI_Resetable.Reset`
  (params (CallingActor :type "Actor Object Reference"))
  (if (> (`KismetArrayLibrary.Array_Length` (`self.Switches`)) 0)
    (`self.Deactivate`)
    (`self.ResetSwitches` (`self.Switches`))
    (if (> (`KismetArrayLibrary.Array_Length` (`self.InputSequence`)) 0)
      (`KismetArrayLibrary.Array_Clear` (`self.SwitchesToReset`))
      (for _array_element (`self.InputSequence`)
        (`KismetArrayLibrary.Array_Add` (`self.SwitchesToReset`) _array_element))
      (for _array_element_2 (`self.SwitchesToReset`)
        (message `/Game/TemplateAssets/Blueprints/UtilityClasses/BPI_Resetable.Reset` _array_element_2 self)))))

(event `self.RemoveFromInputSequence`
  (params (SwitchToRemove :type "/Game/TemplateAssets/Blueprints/BP_Switch Object Reference"))
  (if (> (`KismetArrayLibrary.Array_Length` (`self.InputSequence`)) 0)
    (for (_array_element _array_index) (`self.InputSequence`)
      (if (== _array_element SwitchToRemove)
        (`KismetArrayLibrary.Array_Remove` (`self.InputSequence`) _array_index)
        (break)))))

(fn `SetStructSettings`)

(fn `UserConstructionScript`)
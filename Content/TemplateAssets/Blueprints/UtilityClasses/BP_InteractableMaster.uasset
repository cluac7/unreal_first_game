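; BP_InteractableMaster is a base actor for objects the player can interact with and that can be reset to their starting placement.
; Interact and StopInteract set or clear the player's InteractingObject reference to this actor.
; Reset releases the object if the player is interacting with it, then teleports it back to the transform saved on BeginPlay, toggling physics simulation off and on around the move.
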(event `self.ReceiveBeginPlay`
  (set `self.OriginalTransform` (`self.GetTransform`)))

(event `self.Interact`
  (params (PlayerReference :type "/Game/TemplateAssets/Blueprints/BP_PlayerCharacter Object Reference"))
  (set `/Game/TemplateAssets/Blueprints/BP_PlayerCharacter.InteractingObject` self PlayerReference))

(event `self.StopInteract`
  (params (PlayerReference :type "/Game/TemplateAssets/Blueprints/BP_PlayerCharacter Object Reference"))
  (set `/Game/TemplateAssets/Blueprints/BP_PlayerCharacter.InteractingObject` null PlayerReference))

(event `/Game/TemplateAssets/Blueprints/UtilityClasses/BPI_Resetable.Reset`
  (params (CallingActor :type "Actor Object Reference"))
  (bind _asbp_player_character (cast `/Game/TemplateAssets/Blueprints/BP_PlayerCharacter` (`GameplayStatics.GetPlayerCharacter` 0)))
  (if (== (`/Game/TemplateAssets/Blueprints/BP_PlayerCharacter.InteractingObject` _asbp_player_character) self)
    (`self.StopInteract` _asbp_player_character))
  (`PrimitiveComponent.SetSimulatePhysics` (`self.StaticMesh`) false)
  (`self.K2_SetActorTransform` (`self.OriginalTransform`) false true)
  (`PrimitiveComponent.SetSimulatePhysics` (`self.StaticMesh`) true))

(fn `UserConstructionScript`)